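; BP_TutorialSelection is a main menu Blueprint that switches between a restaurant view and a food view, apparently for tutorial selection.
; SwapToRestaurantCamera and SwapToFoodCamera each activate one capture component, deactivate the other, and print a debug string.
; The Event Graph holds only disconnected copies of the same toggle logic, so switching relies on external calls to the two functions.
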(fn ConstructionScript)

(fn SwaptoFoodCamera
  (Components|Activation|SetActive (Variables|Default|GetRestarauntCapture) false false)
  (Components|Activation|SetActive (Variables|Food|GetFoodCapture) true false)
  (Development|PrintString "fud")
  (return self))

(fn SwaptoRestaurantCamera
  (Components|Activation|SetActive (Variables|Default|GetRestarauntCapture) true false)
  (Components|Activation|SetActive (Variables|Food|GetFoodCapture) false false)
  (Development|PrintString "Res")
  (return self))