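; Player character Blueprint that manages which actors a held-item capture renders and carries a debug check for order rewards.
; ToggleItemShown adds the held item and two nested passes of its attached actors to the capture's show-only list, or clears that list when no valid item is held.
; The T key prints which additional items of the OrderManager's reward at key 0 also appear in its FoundReward.
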(event EventBeginPlay)

(event Collision|EventActorBeginOverlap
  (params (OtherActor :type Actor%20Object%20Reference)))

(event EventTick
  (params (DeltaSeconds :type Float%20%28single-precision%29)))

(event EventToggleItemShown
  (bind _helditem (Variables|Default|GetHeldItem))
  (Utilities|IsValid (Variables|Default|GetHeldItem)
    (:Is%20Valid
      (Utilities|Array|Add (Variables|/Script/Engine.SceneCaptureComponent|GetShowOnlyActors (Variables|Default|GetHeldItemCapture)) _helditem)
      (for _array_element (Actor|GetAttachedActors _helditem true)
        (Utilities|Array|Add (Variables|/Script/Engine.SceneCaptureComponent|GetShowOnlyActors (Variables|Default|GetHeldItemCapture)) _array_element)
        (for _array_element_2 (Actor|GetAttachedActors _array_element true)
          (Utilities|Array|Add (Variables|/Script/Engine.SceneCaptureComponent|GetShowOnlyActors (Variables|Default|GetHeldItemCapture)) _array_element_2))))
    (:Is%20Not%20Valid
      (Utilities|Array|Clear (Variables|/Script/Engine.SceneCaptureComponent|GetShowOnlyActors (Variables|Default|GetHeldItemCapture))))))

(event Input|KeyboardEvents|T
  (params (Key :type Key%20Structure :default "None"))
  (:Pressed
    (bind _outactors (Actor|GetAllActorsOfClass "/Script/FoodGame.OrderManager"))
    (for _array_element (.additionalitems (.Value (Utilities|Map|Find (Variables|/Script/FoodGame.OrderManager|GetRewards (Utilities|Array|Get(acopy) _outactors)) 0)))
      (if (Utilities|Array|ContainsItem (.AdditionalItems (Utilities|Struct|BreakOrderReward (Variables|/Script/FoodGame.OrderManager|GetfoundReward (Utilities|Array|Get(acopy) _outactors)))) _array_element)
        (Development|PrintString (Utilities|String|ToString(Text) (Utilities|Text|FormatText "Yes, FoundReward conatins {x}" _array_element)))))))

(fn ConstructionScript)